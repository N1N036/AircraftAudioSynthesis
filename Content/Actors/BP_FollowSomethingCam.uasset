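; Trackside-style camera pawn that follows an actor, typically an aircraft, and takes player control during flight replay when the target enters its sphere.
; The trigger uses a distance check because collision disrupts JSBSim.
; Tick smoothly aims the shaking camera, sets focus to target distance and narrows FOV non-linearly with distance, previewed in the construction script.
; Outside replay, aircraft targets make it reveal its sphere and draw a debug marker.
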(event `self.ReceiveBeginPlay`
  (bind _returnvalue (`self.GetComponentByClass` (`self.WillLookAtActor`) "/Script/ProjectFanblade.AircraftFlightRecordComponent"))
  (`|ExecutionSequence`
    (:`then_0`
      (if (`self.Dissable`)
        (`self.K2_DestroyActor`)))
    (:`then_1`
      (`CameraShakeSourceComponent.StartCameraShake` :`self` (`self.CameraShakeSource`) :`InCameraShake` "/Script/GameplayCameras.DefaultCameraShakeBase")
      (`/Engine/EditorBlueprintResources/StandardMacros.IsValid` _returnvalue
        (:`Is Valid`
          (if (not (`|EnumEquality` (`AircraftFlightRecordComponent.CurrentMode` _returnvalue) "Replay"))
            (`KismetSystemLibrary.DrawDebugSphere` (`self.K2_GetActorLocation` self) 1000.0 5 (struct :`R` 0.084921 :`G` 1.0 :`A` 1.0) 1000000000.0)
            (`SceneComponent.SetHiddenInGame` (`self.Sphere`) false false)))))))

(event `self.ReceiveTick`
  (params (DeltaSeconds :type "Float (single-precision)"))
  (bind _cinecamera (`self.CineCamera`))
  (bind _cinecamera_2 (`self.CineCamera`))
  (bind _returnvalue (`self.K2_GetActorLocation` (`self.WillLookAtActor`)))
  (bind _returnvalue_2 (`SceneComponent.K2_GetComponentLocation` _cinecamera))
  (bind (_focussettings_focusmethod _focussettings_manualfocusdistance _focussettings_trackingfocussettings _focussettings_bsmoothfocuschanges _focussettings_focussmoothinginterpspeed _focussettings_focusoffset) (break `CameraFocusSettings` (`CineCameraComponent.FocusSettings` _cinecamera_2)))
  (bind _returnvalue_3 (- _returnvalue _returnvalue_2))
  (`|ExecutionSequence`
    (:`then_0`
      (if (`self.CheckIfLookatActorIsIntriggerBox`)
        (if (not (`self.IsPlayerControlled` self))
          (`Controller.Possess` (`GameplayStatics.GetPlayerController` 0) self))))
    (:`then_1`
      (bind _output_get (set `self.NewVar` (`KismetMathLibrary.RLerp` (`self.NewVar`) (`KismetMathLibrary.FindLookAtRotation` _returnvalue_2 _returnvalue) (* DeltaSeconds 8.0) true)))
      (`SceneComponent.K2_SetWorldRotation` (`self.CameraShakeSource`) _output_get false false)
      (set `CineCameraComponent.FocusSettings` (make `CameraFocusSettings` _focussettings_focusmethod (`KismetMathLibrary.VSize` _returnvalue_3) _focussettings_trackingfocussettings _focussettings_bsmoothfocuschanges _focussettings_focussmoothinginterpspeed _focussettings_focusoffset) _cinecamera_2)
      (`CameraComponent.SetFieldOfView` _cinecamera (`KismetMathLibrary.MapRangeClamped` (`KismetMathLibrary.MultiplyMultiply_FloatFloat` (`KismetMathLibrary.MapRangeClamped` (`KismetMathLibrary.VSize` _returnvalue_3) 0.0 400000.0 0.0 1.0) 0.2) 0.0 1.0 90.0 0.1)))))

(fn `CheckIfLookatActorIsIntriggerBox`
  (returns (NewParam :type Boolean))
  (bind _sphere (`self.Sphere`))
  (bind _willlookatactor (`self.WillLookAtActor`))
  (bind _returnvalue (`self.GetComponentByClass` _willlookatactor "/Script/ProjectFanblade.AircraftFlightRecordComponent"))
  (`/Engine/EditorBlueprintResources/StandardMacros.IsValid` _returnvalue
    (:`Is Valid`
      (return (and (`|EnumEquality` (`AircraftFlightRecordComponent.CurrentMode` _returnvalue) "Replay") (< (`KismetMathLibrary.Vector_Distance` (`self.K2_GetActorLocation` _willlookatactor) (`SceneComponent.K2_GetComponentLocation` _sphere)) (`SphereComponent.GetScaledSphereRadius` _sphere)))))))

(fn `UserConstructionScript`
  (bind _cinecamera (`self.CineCamera`))
  (bind _cinecamera_2 (`self.CineCamera`))
  (bind _returnvalue (`self.K2_GetActorLocation` (`self.WillLookAtActor`)))
  (bind _returnvalue_2 (`SceneComponent.K2_GetComponentLocation` _cinecamera))
  (bind (_focussettings_focusmethod _focussettings_manualfocusdistance _focussettings_trackingfocussettings _focussettings_bsmoothfocuschanges _focussettings_focussmoothinginterpspeed _focussettings_focusoffset) (break `CameraFocusSettings` (`CineCameraComponent.FocusSettings` _cinecamera_2)))
  (bind _returnvalue_3 (- _returnvalue _returnvalue_2))
  (`SceneComponent.K2_SetWorldRotation` (`self.CameraShakeSource`) (`KismetMathLibrary.FindLookAtRotation` _returnvalue_2 _returnvalue) false false)
  (set `CineCameraComponent.FocusSettings` (make `CameraFocusSettings` _focussettings_focusmethod (`KismetMathLibrary.VSize` _returnvalue_3) _focussettings_trackingfocussettings _focussettings_bsmoothfocuschanges _focussettings_focussmoothinginterpspeed _focussettings_focusoffset) _cinecamera_2)
  (`CameraComponent.SetFieldOfView` _cinecamera (`KismetMathLibrary.MapRangeClamped` (`KismetMathLibrary.MultiplyMultiply_FloatFloat` (`KismetMathLibrary.MapRangeClamped` (`KismetMathLibrary.VSize` _returnvalue_3) 0.0 400000.0 0.0 1.0) 0.2) 0.0 1.0 90.0 0.1)))