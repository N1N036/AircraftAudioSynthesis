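; Debug helper actor that toggles sonic propagation debug drawing on a watched aircraft during flight replay.
; Each tick it checks whether the target actor's flight recorder is in Replay mode and its location lies inside the trigger box.
; When it does, it copies its DrawDebug setting onto the aircraft's SonicPropagationAudioComponent.
; A point-in-box test replaces overlap events because collision disrupts the JSBSim component.
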(event `self.ReceiveTick`
  (params (DeltaSeconds :type "Float (single-precision)"))
  (if (`self.CheckIfLookatActorIsIntriggerBox`)
    (bind _asaircraft (cast `Aircraft` (`self.WillLookAtActor`)))
    (bind _returnvalue (`self.GetComponentByClass` _asaircraft "/Script/ProjectFanblade.SonicPropagationAudioComponent"))
    (`/Engine/EditorBlueprintResources/StandardMacros.IsValid` _returnvalue
      (:`Is Valid`
        (set `SonicPropagationAudioComponent.bDrawDebug` (`self.Draw Debug`) _returnvalue)))))

(event `self.ReceiveBeginPlay`)

(fn `CheckIfLookatActorIsIntriggerBox`
  (returns (NewParam :type Boolean))
  (bind _triggerbox (`self.TriggerBox`))
  (bind _willlookatactor (`self.WillLookAtActor`))
  (bind _returnvalue (`self.GetComponentByClass` _willlookatactor "/Script/ProjectFanblade.AircraftFlightRecordComponent"))
  (`/Engine/EditorBlueprintResources/StandardMacros.IsValid` _returnvalue
    (:`Is Valid`
      (return (and (`|EnumEquality` (`AircraftFlightRecordComponent.CurrentMode` _returnvalue) "Replay") (`KismetMathLibrary.IsPointInBox` (`self.K2_GetActorLocation` _willlookatactor) (`SceneComponent.K2_GetComponentLocation` _triggerbox) (`BoxComponent.GetScaledBoxExtent` _triggerbox)))))))

(fn `UserConstructionScript`)