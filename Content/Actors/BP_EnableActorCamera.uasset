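; Trigger actor that hands player 0's possession to its WillLookAtActor pawn when that aircraft is inside the box during flight replay.
; Each Tick it checks that the actor's AircraftFlightRecordComponent is in Replay mode and that its location lies within TriggerBox.
; The manual point-in-box test replaces collision overlaps, which interfere with the JSBSim component.
; A Dissable flag destroys the actor at BeginPlay.
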(event `self.ReceiveTick`
  (params (DeltaSeconds :type "Float (single-precision)"))
  (if (`self.CheckIfLookatActorIsIntriggerBox`)
    (bind _aspawn (cast `Pawn` (`self.WillLookAtActor`)))
    (`Controller.Possess` (`GameplayStatics.GetPlayerController` 0) _aspawn)))

(event `self.ReceiveBeginPlay`
  (if (`self.Dissable`)
    (`self.K2_DestroyActor`)))

(fn `CheckIfLookatActorIsIntriggerBox`
  (returns (NewParam :type Boolean))
  (bind _triggerbox (`self.TriggerBox`))
  (bind _willlookatactor (`self.WillLookAtActor`))
  (bind _returnvalue (`self.GetComponentByClass` _willlookatactor "/Script/ProjectFanblade.AircraftFlightRecordComponent"))
  (`/Engine/EditorBlueprintResources/StandardMacros.IsValid` _returnvalue
    (:`Is Valid`
      (return (and (`|EnumEquality` (`AircraftFlightRecordComponent.CurrentMode` _returnvalue) "Replay") (`KismetMathLibrary.IsPointInBox` (`self.K2_GetActorLocation` _willlookatactor) (`SceneComponent.K2_GetComponentLocation` _triggerbox) (`BoxComponent.GetScaledBoxExtent` _triggerbox)))))))

(fn `UserConstructionScript`)