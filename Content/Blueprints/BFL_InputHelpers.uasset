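; Input helper function library whose PrioritizeDualUserInput merges an absolute controller axis and an incremental keyboard axis into one clamped value.
; A changed controller value takes priority and overwrites the output.
; Otherwise, keyboard input shifts the previous output at a rate set by full-change duration, then a per-call loss multiplier applies, unscaled by delta time.
; A by-reference SDualInputCommand struct holds tuning and state between frames.
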(fn `PrioritizeDualUserInput`
  (params (DeltaSeconds :type "Float (double-precision) (by ref)") (ControllerAxis :type "Float (double-precision)") (KeyboardIncDecAxis :type "Float (double-precision)") (DataStructure :type "/Game/Blueprints/S_DualInputCommand Structure (by ref)"))
  (returns (Output :type "Float (double-precision)"))
  (locals (DecreaseSpeed :type "Float (double-precision)") (IncreaseSpeed :type "Float (double-precision)") (Min :type "Float (double-precision)") (Max :type "Float (double-precision)"))
  (bind ((`FullChangeDurationSec_6_7CD37FFE49F95C77D6D63EBCD759328A` _fullchangedurationsec) (`LastControllerValue_10_E69007014700F85933AB3BA0098D8381` _lastcontrollervalue) (`FinalValue_12_1A3A7304475D7438E36342B96684D343` _finalvalue)) (break `/Game/Blueprints/S_DualInputCommand` DataStructure))
  (bind (_fullchangedurationsec_2 _minvalue _maxvalue) (break `/Game/Blueprints/S_DualInputCommand` DataStructure))
  (bind ((`MinValue_9_25AAABEC427A3E51B536609FC8ED6169` _minvalue_2) (`MaxValue_8_37368F5E4DA6DEB8E1BE898072BB1E82` _maxvalue_2)) (break `/Game/Blueprints/S_DualInputCommand` DataStructure))
  ;[1 1 1] Did the Controller Axis value change since last frame ?
  (if (!= ControllerAxis _lastcontrollervalue)
    ;[1 1 1] Yes - Priority to the controller - Keep new value, eventually clamp the controller value, and return it as output value.
    (setmembers `/Game/Blueprints/S_DualInputCommand` :`StructRef` DataStructure :`LastControllerValue` (`local.ControllerAxis`))
    (bind _structout (setmembers `/Game/Blueprints/S_DualInputCommand` :`StructRef` DataStructure :`FinalValue` (`KismetMathLibrary.FClamp` (`local.ControllerAxis`) _minvalue_2 _maxvalue_2)))
    (return (`.FinalValue_12_1A3A7304475D7438E36342B96684D343` (break `/Game/Blueprints/S_DualInputCommand` _structout)))
    (else
      ;[1 1 1] Clamp and return
      (bind _structout_2 (setmembers `/Game/Blueprints/S_DualInputCommand` :`StructRef` DataStructure :`FinalValue` (`KismetMathLibrary.FClamp` (* (+ (* (/ DeltaSeconds _fullchangedurationsec) (`local.KeyboardIncDecAxis`)) _finalvalue) (`.ReturnTo_0_Losses_17_A721744B4BEB586F5A218296470E148F` (break `/Game/Blueprints/S_DualInputCommand` DataStructure))) _minvalue _maxvalue)))
      (return (`.FinalValue_12_1A3A7304475D7438E36342B96684D343` (break `/Game/Blueprints/S_DualInputCommand` _structout_2))))))